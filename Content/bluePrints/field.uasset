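; Game board actor for a SameGame-style puzzle that spawns a checkered cell grid with randomly colored items tracked by grid coordinate.
; Clicking an item runs a breadth-first flood fill and destroys its same-color group if larger than one.
; Remaining items then drop into gaps and shift along X to close empty columns.
; An empty board opens the win menu, while no matching neighbors left opens the lose menu.
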(event EventBeginPlay
  (CallFunction|SpawnCells)
  (Components|DestroyComponent (Variables|Default|GetPlane))
  (CallFunction|SpawnItems))

(fn ConstructionScript)

(fn SpawnCell
  (params (XY :type Int%20Point%20Structure))
  (bind (_x _y) (Utilities|Struct|BreakIntPoint XY))
  (bind _location (CallFunction|XYtoLocation XY))
  (bind _returnvalue (Game|SpawnActorfromClass "/Game/bluePrints/Cells.Cells_C" (Math|Transform|MakeTransform _location) "Undefined" 0 0))
  (Default|SetMaterial _returnvalue (== (Math|Integer|%(Integer) (+ _x _y) 2) 0))
  (return _returnvalue))

(fn SpawnCells
  (bind _xy (Utilities|EnumerateCoords)
    (:LoopBody
      (CallFunction|SpawnCell _xy))))

(fn XYtoLocation
  (params (XY :type Int%20Point%20Structure))
  (bind (_x _y) (Utilities|Struct|BreakIntPoint XY))
  (return (- (* (Math|Vector|MakeVector (Math|Conversions|ToFloat(Integer) _x) (Math|Conversions|ToFloat(Integer) _y) 0.0) (Variables|Default|GetcellSize)) (- (/ (* (Variables|Default|Getsize) (Variables|Default|GetcellSize)) 2.0) (/ (Variables|Default|GetcellSize) 2.0)))))

(fn SpawnItems
  (bind _xy (Utilities|EnumerateCoords)
    (:LoopBody
      (bind _location (CallFunction|XYtoLocation _xy))
      (bind _returnvalue (Game|SpawnActorfromClass "/Game/bluePrints/Item.Item_C" (Math|Conversions|ToTransform(Vector) _location) "Undefined" 0 (Math|Random|RandomIntegerinRange 0 2) self 0))
      (Utilities|Map|Add (Variables|Default|GetItems) _xy _returnvalue))))

(fn OnitemClick
  (params (item :type Item%20Object%20Reference))
  (bind _items (Variables|Default|GetItems))
  (bind _xy (CallFunction|ItemtoXY item))
  (bind _paintedarray (CallFunction|Paint _xy))
  (if (> (Utilities|Array|Length _paintedarray) 1)
    (for _array_element _paintedarray
      (Actor|DestroyActor (.Value (Utilities|Map|Find _items _array_element)))
      (Utilities|Map|Remove _items _array_element))
    (CallFunction|DropItems)
    (CallFunction|FillEmptyColumns)
    (CallFunction|CheckEndGame)))

(fn ItemtoXY
  (params (item :type Item%20Object%20Reference))
  (bind _xy (Utilities|EnumerateCoords)
    (:LoopBody
      (if (== (.Value (Utilities|Map|Find (Variables|Default|GetItems) _xy)) item)
        (LocalVariables|SetResult _xy)))
    (:complete
      (return (LocalVariables|GetResult)))))

(fn Paint
  (params (XY :type Int%20Point%20Structure))
  (bind _paintmap (LocalVariables|GetPaintMap))
  (bind _queue (LocalVariables|GetQueue))
  (bind _output_get (LocalVariables|SetOurXY XY))
  (LocalVariables|SetOurColor (Variables|/Game/bluePrints/Item.Item_C|GetColor (.Value (Utilities|Map|Find (Variables|Default|GetItems) _output_get))))
  (bind _xy (Utilities|EnumerateCoords)
    (:LoopBody
      (Utilities|Map|Add (LocalVariables|GetPaintMap) _xy (LocalVariables|Getinfinite)))
    (:complete
      (Utilities|Array|Add (LocalVariables|GetQueue) (LocalVariables|GetOurXY))
      (Utilities|Map|Add (LocalVariables|GetPaintMap) (LocalVariables|GetOurXY) 0)
      (while (Utilities|Array|IsNotEmpty (LocalVariables|GetQueue))
        (bind _output_get_2 (LocalVariables|SetOurXY (Utilities|Array|Get(acopy) _queue)))
        (Utilities|Array|RemoveIndex _queue)
        (bind _neighbourxy (Utilities|EnumerateNeighboursOfColor _output_get_2 (LocalVariables|GetOurColor))
          (:Loop
            (if (> (.Value (Utilities|Map|Find _paintmap _neighbourxy)) (+ (.Value (Utilities|Map|Find _paintmap (LocalVariables|GetOurXY))) 1))
              (Utilities|Map|Add (LocalVariables|GetPaintMap) _neighbourxy (+ (.Value (Utilities|Map|Find _paintmap (LocalVariables|GetOurXY))) 1))
              (Utilities|Array|Add (LocalVariables|GetQueue) _neighbourxy)))))
      (bind _xy_2 (Utilities|EnumerateCoords)
        (:LoopBody
          (if (< (.Value (Utilities|Map|Find (LocalVariables|GetPaintMap) _xy_2)) (LocalVariables|Getinfinite))
            (Utilities|Array|Add (LocalVariables|GetResult) _xy_2)))
        (:complete
          (return (LocalVariables|GetResult)))))))

(fn TryDrop
  (bind _xy (Utilities|EnumerateCoords)
    (:LoopBody
      (bind _output_get (LocalVariables|SetOldXY _xy))
      (bind _output_get_2 (LocalVariables|SetNewXY (+ _output_get (Class|KismetMathLibrary|IntPointUp))))
      (if (.ReturnValue (Utilities|Map|Find (Variables|Default|GetItems) _output_get))
        (bind _empty (CallFunction|IsCellEmpty _output_get_2))
        (if _empty
          (bind _output_get_3 (LocalVariables|SetItem (.Value (Utilities|Map|Find (Variables|Default|GetItems) (LocalVariables|GetOldXY)))))
          (Utilities|Map|Add (Variables|Default|GetItems) (LocalVariables|GetNewXY) _output_get_3)
          (Utilities|Map|Remove (Variables|Default|GetItems) (LocalVariables|GetOldXY))
          (bind _location (CallFunction|XYtoLocation (LocalVariables|GetNewXY)))
          (Default|EventonSetLocation (LocalVariables|GetItem) _location)
          (LocalVariables|SetResult true))))
    (:complete
      (return (LocalVariables|GetResult)))))

(fn IsCellEmpty
  (params (XY :type Int%20Point%20Structure))
  (bind (_x _y) (Utilities|Struct|BreakIntPoint XY))
  (bind _size (Variables|Default|Getsize))
  (return (Math|Boolean|ANDBoolean (not (.ReturnValue (Utilities|Map|Find (Variables|Default|GetItems) XY))) (Math|Integer|InRange(Integer) _x 0 _size true false) (Math|Integer|InRange(Integer) _y 0 _size true false))))

(fn DropItems
  (while (LocalVariables|GetAreColumnsDropable)
    (bind _success (CallFunction|TryDrop))
    (LocalVariables|SetAreColumnsDropable _success)))

(fn IsСolumnEmpty
  (params (ColumnX :type Integer))
  (LocalVariables|SetResult true)
  (bind _index (Utilities|FlowControl|ForLoopwithBreak 0 (- (Variables|Default|Getsize) 1) :!label _label)
    (:LoopBody
      (bind _empty (CallFunction|IsCellEmpty (Utilities|Struct|MakeIntPoint ColumnX _index)))
      (if (not _empty)
        (LocalVariables|SetResult false)
        (goto _label Break)))
    (:Completed
      (return (LocalVariables|GetResult)))))

(fn FillEmptyColumns
  (bind _index (Utilities|FlowControl|ForLoopwithBreak 0 (- (Variables|Default|Getsize) 1))
    (:LoopBody
      (bind _output_get (LocalVariables|SetEmptyColumnX _index))
      (bind _empty (CallFunction|IsСolumnEmpty _output_get))
      (if _empty
        (Development|PrintString (Utilities|String|BuildString(Integer) "Column " "" (LocalVariables|GetEmptyColumnX) "is empty"))
        (CallFunction|ShiftRightItemstoLeft (LocalVariables|GetEmptyColumnX) (LocalVariables|GetEmptyColumnX))))))

(fn ShiftRightItemstoLeft
  (params (RightFromX :type Integer) (TargetX :type Integer))
  (for _index (range 1 RightFromX)
    (for _index_2 (range 0 (- (Variables|Default|Getsize) 1))
      (bind _output_get (LocalVariables|SetOld%20XY (Utilities|Struct|MakeIntPoint (- RightFromX _index) _index_2)))
      (LocalVariables|SetNew%20XY (Utilities|Struct|MakeIntPoint (+ (- RightFromX _index) 1) _index_2))
      (if (.ReturnValue (Utilities|Map|Find (Variables|Default|GetItems) _output_get))
        (bind _output_get_2 (LocalVariables|SetItem (.Value (Utilities|Map|Find (Variables|Default|GetItems) _output_get))))
        (Utilities|Map|Add (Variables|Default|GetItems) (LocalVariables|GetNew%20XY) _output_get_2)
        (Utilities|Map|Remove (Variables|Default|GetItems) (LocalVariables|GetOld%20XY))
        (bind _location (CallFunction|XYtoLocation (LocalVariables|GetNew%20XY)))
        (Default|EventonSetLocation (LocalVariables|GetItem) _location)))))

(fn CheckEndGame
  (bind _items (Variables|Default|GetItems))
  (Math|Integer|CompareInt (Utilities|Map|Length (Variables|Default|GetItems))
    (:>
      (LocalVariables|SetNeighborCounter 0)
      (bind _keys (Utilities|Map|Keys _items))
      (for _array_element _keys
        (Utilities|EnumerateNeighboursOfColor _array_element (Variables|/Game/bluePrints/Item.Item_C|GetColor (.Value (Utilities|Map|Find _items _array_element)))
          (:Loop
            (LocalVariables|SetNeighborCounter (+ (LocalVariables|GetNeighborCounter) 1)))))
      (Development|PrintString (Utilities|String|BuildString(Integer) "Neightbours " "" (LocalVariables|GetNeighborCounter)))
      (Math|Integer|CompareInt (LocalVariables|GetNeighborCounter) 1
        (:<
          (Game|OpenLevel(byObjectReference) "/Game/maps/LoseGameMenu.LoseGameMenu"))))
    (:==
      (Game|OpenLevel(byObjectReference) "/Game/maps/WinGameMenu.WinGameMenu"))))