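; Item is a clickable colored sphere piece that belongs to a Field, apparently for a board-style game.
; On BeginPlay it picks a blue, green, red or yellow material from its Color value.
; Clicks are forwarded to Field.OnitemClick with itself as the argument, and OnSetLocation eases the root component to a target relative location over a short move.
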(event Custom|Event%20OnSetLocation
  (params (Target%20Location :type Vector))
  (Components|MoveComponentTo (Variables|Transformation|GetRootComponent self) Target%20Location "0, 0, 0" true false 0.4 false))

(event EventBeginPlay
  (bind _sphere (Variables|Default|GetSphere))
  (switch int (Variables|Default|GetColor)
    (:0
      (Rendering|Material|SetMaterial _sphere 0 "/Game/Materials/Blue.Blue"))
    (:1
      (Rendering|Material|SetMaterial _sphere 0 "/Game/Materials/green.green"))
    (:2
      (Rendering|Material|SetMaterial _sphere 0 "/Game/Materials/red.red"))
    (:3
      (Rendering|Material|SetMaterial _sphere 0 "/Game/Materials/Yellow.Yellow"))))

(event MouseInput|EventActorOnClicked
  (params (ButtonPressed :type Key%20Structure :default "None"))
  (Default|OnitemClick (Variables|Default|GetField) self))

(fn ConstructionScript)